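; BP_CurvedStairs is a generated dynamic mesh actor that builds a procedural curved staircase as a placeable tool.
; On rebuild, it appends curved stairs from Geometry Script to the target mesh, driven by variables for step size, inner radius, curve angle, step count and a floating option.
; It then enables complex-as-simple collision on the dynamic mesh component, and the construction script only calls its parent.
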(event `self.OnRebuildGeneratedMesh`
  (params (TargetMesh :type "DynamicMesh Object Reference"))
  ;[1 1 1] Curved Stair creation
  (set `self.DynamicMesh` TargetMesh)
  (`GeometryScriptLibrary_MeshPrimitiveFunctions.AppendCurvedStairs` (`self.DynamicMesh`) (struct) (struct) (`self.Step Width`) (`self.Step Height`) (`self.Inner Radius`) (`self.Curve Angle`) (`self.Num Steps`) (`self.Floating`) null)
  (`DynamicMeshComponent.EnableComplexAsSimpleCollision` (`self.DynamicMeshComponent`)))

(fn `UserConstructionScript`
  (`parent.UserConstructionScript`))