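; Base actor for a mesh baking tool that turns Geometry Script dynamic meshes into static mesh assets.
; The construction script shows either the editable dynamic mesh or the baked TargetStaticMesh, based on Editable.
; GenerateNewStaticMesh creates a uniquely named game or plugin asset, while BakeToStaticMesh overwrites the target; both copy materials and collision.
; Rebuild only resets to a cube, material hooks are empty, and CleanDegenerateTris optionally deletes near-zero-area triangles.
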(event `ClearMaterials`)

(event `self.OnRebuildGeneratedMesh`
  (params (TargetMesh :type "DynamicMesh Object Reference"))
  (`DynamicMesh.ResetToCube` TargetMesh))

(fn `ApplyMaterials`
  (params (Materials :type "Array of MaterialInterface Object Reference")))

(fn `BakeToStaticMesh`
  (bind _targetstaticmesh (`self.TargetStaticMesh`))
  (bind _returnvalue (`BaseDynamicMeshComponent.GetDynamicMesh` (`self.DynamicMeshComponent`)))
  (`GeometryScriptLibrary_StaticMeshFunctions.CopyMeshToStaticMesh` _returnvalue _targetstaticmesh (make `GeometryScriptCopyMeshToAssetOptions` false false false false _ _ true (make `GeometryScriptNaniteOptions` (`self.Enable Nanite`) (`self.NaniteFallBackPercent`))) (struct) null
    (:`Success`
      (for (_array_element _array_index) (`MeshComponent.GetMaterials` (`self.DynamicMeshComponent`))
        (`StaticMesh.SetMaterial` _targetstaticmesh _array_index _array_element))
      (`GeometryScriptLibrary_CollisionFunctions.SetStaticMeshCollisionFromComponent` _targetstaticmesh (`self.DynamicMeshComponent`) (make `GeometryScriptSetSimpleCollisionOptions` true) null))))

(fn `CleanDegenerateTris`
  (params (Mesh :type "DynamicMesh Object Reference") (SafeNormalTolerance :type "Float (double-precision)" :default 0.0005) (DebugLogCount :type Boolean) (DeleteDegenerates :type Boolean :default true))
  (locals (DegenerateTriList :type "Array of Integer"))
  (bind _triangleidlist (`GeometryScriptLibrary_MeshQueryFunctions.GetAllTriangleIDs` Mesh))
  (bind _indexarray (`GeometryScriptLibrary_ListUtilityFunctions.ConvertIndexListToArray` _triangleidlist))
  (for _array_element _indexarray
    (bind (_bisvalidtriangle _vertex1 _vertex2 _vertex3) (`GeometryScriptLibrary_MeshQueryFunctions.GetTrianglePositions` (`local.Mesh`) _array_element))
    (`/Engine/EditorBlueprintResources/StandardMacros.CompareFloat` (`KismetMathLibrary.VSizeSquared` (`KismetMathLibrary.Cross_VectorVector` (- _vertex3 _vertex1) (- _vertex2 _vertex1))) (`local.SafeNormalTolerance`)
      (:`<`
        (`KismetArrayLibrary.Array_Add` (`local.DegenerateTriList`) _array_element))))
  (if (not (`KismetArrayLibrary.Array_IsEmpty` (`local.DegenerateTriList`)))
    (`|ExecutionSequence`
      (:`then_0`
        (if (`local.DebugLogCount`)
          (`KismetSystemLibrary.PrintString` (`KismetStringLibrary.Concat_StrStr` (`KismetStringLibrary.Concat_StrStr` "Found " (`KismetStringLibrary.Conv_IntToString` (`KismetArrayLibrary.Array_Length` (`local.DegenerateTriList`)))) " Degenerates"))))
      (:`then_1`
        (if (`local.DeleteDegenerates`)
          (bind _indexlist (`GeometryScriptLibrary_ListUtilityFunctions.ConvertArrayToIndexList` (`local.DegenerateTriList`) "Triangle"))
          (bind (_numdeleted _returnvalue) (`GeometryScriptLibrary_MeshBasicEditFunctions.DeleteTrianglesFromMesh` (`local.Mesh`) _indexlist))
          (`GeometryScriptLibrary_MeshRepairFunctions.CompactMesh` _returnvalue null))))))

(fn `GenerateNewStaticMesh`
  (bind _dynamicmeshcomponent (`self.DynamicMeshComponent`))
  (bind _returnvalue (`KismetTextLibrary.Conv_TextToString` (`|FormatText` "{PathSource}/{FullPath}" (`KismetMathLibrary.SelectString` (`KismetStringLibrary.Concat_StrStr` "/" (`self.PluginName`)) "/Game" (`self.bIsInPlugin`)) (`self.PathName`))))
  (bind _returnvalue_2 (`KismetMathLibrary.SelectString` (`KismetStringLibrary.Concat_StrStr` _returnvalue "/Generated") _returnvalue (`self.bGeneratedSubFolder`)))
  (set `self.SourceGeneratorKey` (`KismetGuidLibrary.Conv_GuidToString` (`KismetGuidLibrary.NewGuid`)))
  (bind _returnvalue_3 (`BaseDynamicMeshComponent.GetDynamicMesh` (`self.DynamicMeshComponent`)))
  (`KismetSystemLibrary.PrintString` _returnvalue_2) ; Print for debug
  (bind _uniqueassetpathandname (`GeometryScriptLibrary_CreateNewAssetFunctions.CreateUniqueNewAssetPathName` _returnvalue_2 (`self.AssetName`) (struct) null)
    (:`Failure`
      (`KismetSystemLibrary.PrintString` "Failed to Create Asset Path"))
    (:`Success`
      (bind _returnvalue_4 (`GeometryScriptLibrary_CreateNewAssetFunctions.CreateNewStaticMeshAssetFromMesh` _returnvalue_3 _uniqueassetpathandname (make `GeometryScriptCreateNewStaticMeshAssetOptions` false false (`self.Enable Nanite`) (struct :`PositionPrecision` -2147483648 :`NormalPrecision` -1 :`TangentPrecision` -1 :`KeepPercentTriangles` 1.0 :`FallbackTarget` "Auto" :`FallbackPercentTriangles` 1.0 :`FallbackRelativeError` 1.0) (`self.NaniteFallBackPercent`) true (`self.Collision Mode`)) null)
        (:`Failure`
          (`KismetSystemLibrary.PrintString` "Failed to Create New Asset"))
        (:`Success`
          (bind _output_get (set `self.TargetStaticMesh` _returnvalue_4))
          (`GeometryScriptLibrary_CollisionFunctions.SetStaticMeshCollisionFromComponent` _output_get _dynamicmeshcomponent (struct :`bEmitTransaction` true) null)
          ;[1 1 1] Add materials
          (for (_array_element _array_index) (`MeshComponent.GetMaterials` _dynamicmeshcomponent)
            (`StaticMesh.SetMaterial` _output_get _array_index _array_element)))))))

(fn `UserConstructionScript`
  (`SceneComponent.SetVisibility` (`self.DynamicMeshComponent`) (`self.Editable`) false)
  (`SceneComponent.SetVisibility` (`self.BakedMesh`) (not (`self.Editable`)) false)
  (`StaticMeshComponent.SetStaticMesh` (`self.BakedMesh`) (`self.TargetStaticMesh`)))