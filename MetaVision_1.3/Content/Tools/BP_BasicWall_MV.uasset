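; BP_BasicWall_MV is a Geometry Script generated mesh actor that builds a parametric wall.
; On rebuild, it appends a box sized by length, thickness and height, with configurable segments along its length and per-face polygroups.
; It then assigns the wall material, scales UVs uniformly and releases compute meshes.
; A custom event clears the wall material, then runs the same build chain.
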(event `CustomEvent`
  (bind _uvscale (`self.UVScale`))
  (set `self.Material Wall` null)
  (set `self.DynamicMesh` (stale `self.OnRebuildGeneratedMesh` TargetMesh) :!label _label)
  ;[1 1 1] Create wall
  (bind _returnvalue (`GeometryScriptLibrary_MeshPrimitiveFunctions.AppendBox` (`self.DynamicMesh`) (make `GeometryScriptPrimitiveOptions` "PerFace") (struct) (`self.Wall Lenght`) (`self.Wall Thickness`) (`self.Wall Height`) (`self.Add Segments`) 0 0 "Base" null))
  (set `self.DynamicMesh` _returnvalue)
  ;[1 1 1] Assign Materials
  (`DynamicMeshComponent.ConfigureMaterialSet` (`self.DynamicMeshComponent`) (`|MakeArray` (`self.Material Wall`)))
  ;[1 1 1] UV Settings
  (`GeometryScriptLibrary_MeshUVFunctions.ScaleMeshUVs` (`self.DynamicMesh`) 0 (`KismetMathLibrary.MakeVector2D` _uvscale _uvscale) (1.0 1.0) (struct) null)
  (`self.ReleaseAllComputeMeshes`))

(event `self.OnRebuildGeneratedMesh`
  (params (TargetMesh :type "DynamicMesh Object Reference"))
  (goto _label))

(fn `UserConstructionScript`
  (`parent.UserConstructionScript`))