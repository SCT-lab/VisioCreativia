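; Procedural sphere tool built on a generated dynamic mesh actor, producing either a full sphere or a hollow dome with Geometry Script.
; On mesh rebuild it appends a lat-long sphere from the radius and slice settings.
; In dome mode it plane-cuts the sphere at the cutter handle, boolean-subtracts a smaller pooled compute-mesh sphere to leave a shell of set thickness, then scales UVs.
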(event `self.OnRebuildGeneratedMesh`
  (params (TargetMesh :type "DynamicMesh Object Reference"))
  (bind _returnvalue (`self.K2_GetActorLocation`))
  (bind _uvscale (`self.UVScale`))
  (set `self.DynamicMesh` TargetMesh)
  ;[1 1 1] Create Sphere A
  (bind _returnvalue_2 (`GeometryScriptLibrary_MeshPrimitiveFunctions.AppendSphereLatLong` (`self.DynamicMesh`) (make `GeometryScriptPrimitiveOptions` "PerFace") (struct) (select `bool` false :`false` (`self.Radius`) :`true` (`KismetMathLibrary.Abs` (`KismetMathLibrary.Vector_Distance2D` (+ (`self.Vector Handle`) _returnvalue) _returnvalue))) (`self.Horizontal Slices`) (`self.Vertical Slices`) "Center" null))
  (set `self.DynamicMesh` _returnvalue_2)
  ;[1 1 1] Custom Cutter
  (if (`self.Is a dome?`)
    (bind _returnvalue_3 (`GeometryScriptLibrary_MeshBooleanFunctions.ApplyMeshPlaneCut` (`self.DynamicMEsh`) (`KismetMathLibrary.MakeTransform` (`self.Cutter Handle`) (`self.Cutter Rotation`)) (make `GeometryScriptMeshPlaneCutOptions` true true true) null))
    (bind _returnvalue_4 (`self.AllocateComputeMesh`))
    ;[1 1 1] Create Mesh B
    (bind _returnvalue_5 (`GeometryScriptLibrary_MeshPrimitiveFunctions.AppendSphereLatLong` _returnvalue_4 (struct) (struct) (- (`self.Radius`) (`self.Sphere Thickness`)) (`self.Horizontal Slices`) (`self.Vertical Slices`) "Center" null))
    (bind _output_get (set `self.Target Mesh` _returnvalue_5))
    ;[1 1 1] Boole A-B
    (bind _returnvalue_6 (`GeometryScriptLibrary_MeshBooleanFunctions.ApplyMeshBoolean` _returnvalue_3 (struct) _output_get (struct) "Subtract" (struct) null))
    ;[1 1 1] UV Settings
    (`GeometryScriptLibrary_MeshUVFunctions.ScaleMeshUVs` _returnvalue_6 0 (`KismetMathLibrary.MakeVector2D` _uvscale _uvscale) (1.0 1.0) (struct) null)
    (`self.ReleaseAllComputeMeshes`)))

(fn `UserConstructionScript`
  (`parent.UserConstructionScript`))