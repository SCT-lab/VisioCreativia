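; Level-building ramp tool that procedurally generates a ramp mesh with Geometry Script, shaped by the TopPoint and FloorPoint vectors.
; On rebuild it extrudes a polygon side profile by TopPoint.Y, cleans degenerate triangles, applies the material and enables complex-as-simple collision.
; It then box-projects UVs using UVScale.
; ClearMaterials empties the material and rebuilds the geometry without that UV pass.
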(event `self.ClearMaterials`
  (bind (_toppoint_x _toppoint_y _toppoint_z) (`KismetMathLibrary.BreakVector` (`self.TopPoint`)))
  (bind _floorpoint_x (`KismetMathLibrary.BreakVector` (`self.FloorPoint`)))
  (bind _dynamicmeshcomponent (`self.DynamicMeshComponent`))
  ;[1 1 1] CLEAR MATERIALS
  (set `self.Material` null)
  (`DynamicMeshComponent.ConfigureMaterialSet` (`self.DynamicMeshComponent`) (`|MakeArray` (`self.Material`)))
  (bind _returnvalue (`BaseDynamicMeshComponent.GetDynamicMesh` (`self.DynamicMeshComponent`) :!label _label))
  (bind _returnvalue_2 (`DynamicMesh.Reset` _returnvalue))
  (bind _output_get (set `self.TargetMesh` _returnvalue_2))
  (bind _returnvalue_3 (`GeometryScriptLibrary_MeshPrimitiveFunctions.AppendTriangulatedPolygon` _output_get (struct) (`KismetMathLibrary.MakeTransform` (`KismetMathLibrary.MakeVector` 0.0 0.0 _toppoint_z) (struct :`Roll` 90.0)) (`|MakeArray` (0.0 0.0) (`KismetMathLibrary.MakeVector2D` 0.0 _toppoint_z) (`KismetMathLibrary.MakeVector2D` _floorpoint_x _toppoint_z) (`KismetMathLibrary.MakeVector2D` _toppoint_x) :!type "Vector2D Structure") true null))
  (bind _returnvalue_4 (`GeometryScriptLibrary_MeshModelingFunctions.ApplyMeshExtrude_Compatibility_5p0` _returnvalue_3 (make `GeometryScriptMeshExtrudeOptions` _toppoint_y (0.0 1.0 0.0)) null))
  (`self.CleanDegenerateTris` _returnvalue_4)
  (`DynamicMeshComponent.ConfigureMaterialSet` _dynamicmeshcomponent (`|MakeArray` (`self.Material`)))
  (`self.ReleaseAllComputeMeshes`)
  (`DynamicMeshComponent.EnableComplexAsSimpleCollision` _dynamicmeshcomponent))

(event `self.OnRebuildGeneratedMesh`
  (params (TargetMesh :type "DynamicMesh Object Reference"))
  (bind _uv_scale (`self.UV Scale`))
  (`|ExecutionSequence`
    (:`then_0`
      (goto _label))
    (:`then_1`
      (`GeometryScriptLibrary_MeshUVFunctions.SetMeshUVsFromBoxProjection` (`self.TargetMesh`) 0 (`KismetMathLibrary.MakeTransform` (0.0 0.0 0.0) (struct) (`KismetMathLibrary.MakeVector` _uv_scale _uv_scale _uv_scale)) (struct) 2 null))))

(event `CustomEvent`)

(fn `UserConstructionScript`
  (`parent.UserConstructionScript`))