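; Procedural Geometry Script tool actor that rebuilds a framed painting or panel mesh, sized by the Handle vector.
; An extruded rounded or rectangular base is booleaned with an inset painting shape carrying material ID 1 for its separate material.
; The Half Half type cuts and rebuilds part of the outline with square corners.
; Optional bevels, plane cut and mirror finish the mesh, along with split normals and degenerate-triangle cleanup.
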(event EventBeginPlay
  (|CallParentFunction) ; This node is disabled and will not be called.\nDrag off pins to build functionality.
)

(event EventTick
  (params (DeltaSeconds :type Float%20%28single-precision%29))
  (|CallParentFunction DeltaSeconds) ; This node is disabled and will not be called.\nDrag off pins to build functionality.
)

(event Events|EventOnRebuildGeneratedMesh
  (params (TargetMesh :type Dynamic%20Mesh%20Object%20Reference))
  (bind (_location _axis) (|GetLocationAndAxis_2_2))
  (bind (_offsetcentery _x _y _z) (|GetInfoCutter_2))
  (bind (_offsetcenterx _offsetcentery_2 _x_2 _y_2 _extrude) (|GetInfoNewCorner_2))
  (bind (_offsetx _offsety _offsetz _x_3 _y_3) (|GetNewPiecesInfos_2))
  (bind (_offsetcenterx_2 _offsetcentery_3 _x_4 _y_4 _cornerradius) (|GetInfosFromVector_2))
  (bind (_offetcenterx _offsetcentery_4 _offsetcenterz _x_5 _y_5 _cornerradius_2) (|GetInfosFromParent_2))
  (bind _returnvalue (DynamicMeshComponent|GetDynamicMesh (Variables|Default|GetDynamicMeshComponent)))
  (bind _returnvalue_2 (DynamicMesh|Reset _returnvalue))
  ;[1 1 1] PanelBase
  (bind _returnvalue_3 (Class|GeometryScriptLibraryMeshPrimitiveFunctions|AppendRoundRectangleCompatibility50 _returnvalue_2 (Utilities|Struct|MakeGeometryScriptPrimitiveOptions "PerFace" false "Uniform") (Math|Transform|MakeTransform (Math|Vector|MakeVector _offsetcenterx_2 _offsetcentery_3 0.0) "0, 0, 0" "1.000000,1.000000,1.000000") _x_4 _y_4 _cornerradius 0 0 (Variables|Settings|GetSteps%20Round) 0))
  (Variables|Default|SetDynamicMEsh _returnvalue_3)
  (if (Variables|Settings|Frame|GetbRectangular?)
    (bind _returnvalue_4 (Class|GeometryScriptLibraryMeshSimplifyFunctions|ApplySimplifytoTriangleCount (Variables|Default|GetDynamicMEsh) 2 (Utilities|Struct|MakeGeometryScriptSimplifyMeshOptions "AttributeAware" true true true false false true) 0))
    (Variables|Default|SetDynamicMEsh _returnvalue_4))
  (bind _returnvalue_5 (Class|GeometryScriptLibraryMeshModelingFunctions|ApplyMeshExtrudeCompatibility5p0 (Variables|Default|GetDynamicMEsh) (Utilities|Struct|MakeGeometryScriptMeshExtrudeOptions (.z (Variables|Settings|Frame|GetHandle)) "0.000000,0.000000,1.000000" 1.0 true) 0))
  (Variables|Default|SetDynamicMEsh _returnvalue_5)
  (if (Variables|Settings|Frame|GetbBevelFrame)
    (bind _target_mesh (CallFunction|FnBevel (Variables|Default|GetDynamicMEsh) (Variables|Settings|Frame|GetBevelDistanceFrame)))
    (Variables|Default|SetDynamicMEsh _target_mesh))
  ;[1 1 1] Topper
  (bind _returnvalue_6 (DynamicMeshActor|AllocateComputeMesh))
  (bind _returnvalue_7 (Class|GeometryScriptLibraryMeshPrimitiveFunctions|AppendRoundRectangleCompatibility50 :TargetMesh _returnvalue_6 :Transform (Math|Transform|MakeTransform (Math|Vector|MakeVector _offetcenterx _offsetcentery_4 _offsetcenterz) "0, 0, 0" "1.000000,1.000000,1.000000") :DimensionX _x_5 :DimensionY _y_5 :CornerRadius _cornerradius_2 :StepsRound (Variables|Settings|GetSteps%20Round) :Debug 0))
  (Variables|Default|SetTarget%20Mesh _returnvalue_7)
  (if (Variables|Settings|Painting|GetbRectangularPainting)
    (bind _returnvalue_8 (Class|GeometryScriptLibraryMeshSimplifyFunctions|ApplySimplifytoTriangleCount (Variables|Default|GetTarget%20Mesh) 2 (Utilities|Struct|MakeGeometryScriptSimplifyMeshOptions "AttributeAware" true true true false false true) 0))
    (Variables|Default|SetTarget%20Mesh _returnvalue_8))
  (bind _returnvalue_9 (Class|GeometryScriptLibraryMeshModelingFunctions|ApplyMeshExtrudeCompatibility5p0 (Variables|Default|GetTarget%20Mesh) (Utilities|Struct|MakeGeometryScriptMeshExtrudeOptions (Variables|Settings|Painting|GetPaintingExtrude) "0.000000,0.000000,1.000000" 1.0 true) 0))
  (GeometryScript|UVs|ScaleMeshUVs :TargetMesh (Variables|Default|GetTarget%20Mesh) :Scale (Math|Vector2D|MakeVector2D (Variables|Settings|UVSettings|GetScale%20X) (Variables|Settings|UVSettings|GetScale%20Y)) :Debug 0)
  (bind _returnvalue_10 (GeometryScript|Materials|EnableMaterialIDs _returnvalue_9 0))
  (bind _returnvalue_11 (GeometryScript|Materials|RemapMaterialIDs _returnvalue_10 0 1 0))
  (Variables|Default|SetTarget%20Mesh _returnvalue_11)
  (if (Variables|Settings|Painting|GetbBevelPainting)
    (bind _target_mesh_2 (CallFunction|FnBevel (Variables|Default|GetTarget%20Mesh) (Variables|Settings|Painting|GetBevelDistancePainting)))
    (Variables|Default|SetTarget%20Mesh _target_mesh_2))
  (bind _returnvalue_12 (GeometryScript|Booleans|ApplyMeshBoolean :TargetMesh _returnvalue_5 :ToolMesh (Variables|Default|GetTarget%20Mesh) :Operation (Variables|Settings|GetOperation) :Debug 0))
  (switch Utilities|FlowControl|Switch|SwitchonEnumMV_PanelType (Variables|Settings|GetType)
    (:NewEnumerator0
      _)
    (:NewEnumerator1
      ;[1 1 1] Different Half
      (bind _returnvalue_13 (DynamicMeshActor|AllocateComputeMesh))
      (bind _returnvalue_14 (Class|GeometryScriptLibraryMeshPrimitiveFunctions|AppendBox :TargetMesh _returnvalue_13 :Transform (Math|Transform|MakeTransform (Math|Vector|MakeVector 0.0 _offsetcentery 0.0) "0, 0, 0" "1.000000,1.000000,1.000000") :DimensionX _x :DimensionY _y :DimensionZ _z :Debug 0))
      (bind _returnvalue_15 (GeometryScript|Booleans|ApplyMeshBoolean :TargetMesh _returnvalue_12 :ToolMesh _returnvalue_14 :Operation "Subtract" :Debug 0))
      (bind _returnvalue_16 (DynamicMeshActor|AllocateComputeMesh))
      (bind _returnvalue_17 (Class|GeometryScriptLibraryMeshPrimitiveFunctions|AppendRectangleCompatibility50 :TargetMesh _returnvalue_16 :Transform (Math|Transform|MakeTransform (Math|Vector|MakeVector _offsetcenterx _offsetcentery_2 0.0) "0, 0, 0" "1.000000,1.000000,1.000000") :DimensionX _x_2 :DimensionY _y_2 :Debug 0))
      (bind _returnvalue_18 (Class|GeometryScriptLibraryMeshModelingFunctions|ApplyMeshExtrudeCompatibility5p0 _returnvalue_17 (Utilities|Struct|MakeGeometryScriptMeshExtrudeOptions _extrude "0.000000,0.000000,1.000000" 1.0 true) 0))
      (bind _returnvalue_19 (GeometryScript|Booleans|ApplyMeshBoolean :TargetMesh _returnvalue_15 :ToolMesh _returnvalue_18 :Operation "Union" :Debug 0))
      (bind _returnvalue_20 (DynamicMeshActor|AllocateComputeMesh))
      (bind _returnvalue_21 (Class|GeometryScriptLibraryMeshPrimitiveFunctions|AppendRectangleCompatibility50 :TargetMesh _returnvalue_20 :Transform (Math|Transform|MakeTransform (Math|Vector|MakeVector _offsetx _offsety _offsetz) "0, 0, 0" "1.000000,1.000000,1.000000") :DimensionX _x_3 :DimensionY _y_3 :Debug 0))
      (bind _returnvalue_22 (Class|GeometryScriptLibraryMeshModelingFunctions|ApplyMeshExtrudeCompatibility5p0 _returnvalue_21 (Utilities|Struct|MakeGeometryScriptMeshExtrudeOptions (Variables|Settings|Painting|GetPaintingExtrude) "0.000000,0.000000,1.000000" 1.0 true) 0))
      (bind _returnvalue_23 (GeometryScript|Materials|EnableMaterialIDs _returnvalue_22 0))
      (bind _returnvalue_24 (GeometryScript|Materials|RemapMaterialIDs _returnvalue_23 0 1 0))
      (GeometryScript|Booleans|ApplyMeshBoolean :TargetMesh _returnvalue_19 :ToolMesh _returnvalue_24 :Operation (Variables|Settings|GetOperation) :Debug 0)))
  (bind _returnvalue_25 (Class|GeometryScriptLibraryMeshNormalsFunctions|ComputeSplitNormals _returnvalue_12 (Utilities|Struct|MakeGeometryScriptSplitNormalsOptions true 25.0 false "(bDefaultLayer=True,ExtendedLayerIndex=0)") (Utilities|Struct|MakeGeometryScriptCalculateNormalsOptions true true) 0))
  (Variables|Default|SetDynamicMEsh _returnvalue_25)
  (if (Variables|Settings|Cutter|GetbCustomCutter)
    ;[1 1 1] Cutter
    (Class|GeometryScriptLibraryMeshBooleanFunctions|ApplyMeshPlaneCut (Variables|Default|GetDynamicMEsh) (Math|Transform|MakeTransform (Variables|Settings|Cutter|GetCustomCutter) (Variables|Settings|Cutter|GetCustomCutterRotation) "1.000000,1.000000,1.000000") (Utilities|Struct|MakeGeometryScriptMeshPlaneCutOptions true true false 1.0) 0))
  (if (Variables|Settings|GetbBevelCombine)
    (CallFunction|FnBevel (Variables|Default|GetDynamicMEsh) (Variables|Settings|GetBevelDistanceCombine)))
  (if (Variables|Settings|Mirror|GetbMirror)
    ;[1 1 1] Mirror
    (bind _returnvalue_26 (Class|GeometryScriptLibraryMeshBooleanFunctions|ApplyMeshMirror (Variables|Default|GetDynamicMEsh) (Math|Transform|MakeTransform _location _axis "1.000000,1.000000,1.000000") (Utilities|Struct|MakeGeometryScriptMeshMirrorOptions true true true) 0))
    (Variables|Default|SetDynamicMEsh _returnvalue_26))
  (CallFunction|CleanDegenerateTris (Variables|Default|GetDynamicMEsh) (Variables|Settings|GetSafe%20Normal%20Tolerance) false true)
  (Class|DynamicMeshComponent|ConfigureMaterialSet (Variables|Default|GetDynamicMeshComponent) (Utilities|Array|MakeArray (Variables|Settings|Frame|GetMaterialFrame) (Variables|Settings|Painting|GetMaterialPainting)))
  (DynamicMeshActor|ReleaseAllComputeMeshes))

(event EventClearMaterials
  (bind (_location _axis) (|GetLocationAndAxis_2_2))
  (bind (_offsetcentery _x _y _z) (|GetInfoCutter_2))
  (bind (_offsetcenterx _offsetcentery_2 _x_2 _y_2 _extrude) (|GetInfoNewCorner_2))
  (bind (_offsetx _offsety _offsetz _x_3 _y_3) (|GetNewPiecesInfos_2))
  (bind (_offsetcenterx_2 _offsetcentery_3 _x_4 _y_4 _cornerradius) (|GetInfosFromVector_2))
  (bind (_offetcenterx _offsetcentery_4 _offsetcenterz _x_5 _y_5 _cornerradius_2) (|GetInfosFromParent_2))
  ;[1 1 1] CLEAR MATERIALS
  (Variables|Settings|Frame|SetMaterialFrame 0)
  (Variables|Settings|Painting|SetMaterialPainting 0)
  (bind _returnvalue (DynamicMeshComponent|GetDynamicMesh (Variables|Default|GetDynamicMeshComponent)))
  (bind _returnvalue_2 (DynamicMesh|Reset _returnvalue))
  ;[1 1 1] PanelBase
  (bind _returnvalue_3 (Class|GeometryScriptLibraryMeshPrimitiveFunctions|AppendRoundRectangleCompatibility50 _returnvalue_2 (Utilities|Struct|MakeGeometryScriptPrimitiveOptions "PerFace" false "Uniform") (Math|Transform|MakeTransform (Math|Vector|MakeVector _offsetcenterx_2 _offsetcentery_3 0.0) "0, 0, 0" "1.000000,1.000000,1.000000") _x_4 _y_4 _cornerradius 0 0 (Variables|Settings|GetSteps%20Round) 0))
  (Variables|Default|SetDynamicMEsh _returnvalue_3)
  (if (Variables|Settings|Frame|GetbRectangular?)
    (bind _returnvalue_4 (Class|GeometryScriptLibraryMeshSimplifyFunctions|ApplySimplifytoTriangleCount (Variables|Default|GetDynamicMEsh) 2 (Utilities|Struct|MakeGeometryScriptSimplifyMeshOptions "AttributeAware" true true true false false true) 0))
    (Variables|Default|SetDynamicMEsh _returnvalue_4))
  (bind _returnvalue_5 (Class|GeometryScriptLibraryMeshModelingFunctions|ApplyMeshExtrudeCompatibility5p0 (Variables|Default|GetDynamicMEsh) (Utilities|Struct|MakeGeometryScriptMeshExtrudeOptions (.z (Variables|Settings|Frame|GetHandle)) "0.000000,0.000000,1.000000" 1.0 true) 0))
  (Variables|Default|SetDynamicMEsh _returnvalue_5)
  (if (Variables|Settings|Frame|GetbBevelFrame)
    (bind _target_mesh (CallFunction|FnBevel (Variables|Default|GetDynamicMEsh) (Variables|Settings|Frame|GetBevelDistanceFrame)))
    (Variables|Default|SetDynamicMEsh _target_mesh))
  ;[1 1 1] Topper
  (bind _returnvalue_6 (DynamicMeshActor|AllocateComputeMesh))
  (bind _returnvalue_7 (Class|GeometryScriptLibraryMeshPrimitiveFunctions|AppendRoundRectangleCompatibility50 :TargetMesh _returnvalue_6 :Transform (Math|Transform|MakeTransform (Math|Vector|MakeVector _offetcenterx _offsetcentery_4 _offsetcenterz) "0, 0, 0" "1.000000,1.000000,1.000000") :DimensionX _x_5 :DimensionY _y_5 :CornerRadius _cornerradius_2 :StepsRound (Variables|Settings|GetSteps%20Round) :Debug 0))
  (Variables|Default|SetTarget%20Mesh _returnvalue_7)
  (if (Variables|Settings|Painting|GetbRectangularPainting)
    (bind _returnvalue_8 (Class|GeometryScriptLibraryMeshSimplifyFunctions|ApplySimplifytoTriangleCount (Variables|Default|GetTarget%20Mesh) 2 (Utilities|Struct|MakeGeometryScriptSimplifyMeshOptions "AttributeAware" true true true false false true) 0))
    (Variables|Default|SetTarget%20Mesh _returnvalue_8))
  (bind _returnvalue_9 (Class|GeometryScriptLibraryMeshModelingFunctions|ApplyMeshExtrudeCompatibility5p0 (Variables|Default|GetTarget%20Mesh) (Utilities|Struct|MakeGeometryScriptMeshExtrudeOptions (Variables|Settings|Painting|GetPaintingExtrude) "0.000000,0.000000,1.000000" 1.0 true) 0))
  (GeometryScript|UVs|ScaleMeshUVs :TargetMesh (Variables|Default|GetTarget%20Mesh) :Scale (Math|Vector2D|MakeVector2D (Variables|Settings|UVSettings|GetScale%20X) (Variables|Settings|UVSettings|GetScale%20Y)) :Debug 0)
  (bind _returnvalue_10 (GeometryScript|Materials|EnableMaterialIDs _returnvalue_9 0))
  (bind _returnvalue_11 (GeometryScript|Materials|RemapMaterialIDs _returnvalue_10 0 1 0))
  (Variables|Default|SetTarget%20Mesh _returnvalue_11)
  (if (Variables|Settings|Painting|GetbBevelPainting)
    (bind _target_mesh_2 (CallFunction|FnBevel (Variables|Default|GetTarget%20Mesh) (Variables|Settings|Painting|GetBevelDistancePainting)))
    (Variables|Default|SetTarget%20Mesh _target_mesh_2))
  (bind _returnvalue_12 (GeometryScript|Booleans|ApplyMeshBoolean :TargetMesh _returnvalue_5 :ToolMesh (Variables|Default|GetTarget%20Mesh) :Operation (Variables|Settings|GetOperation) :Debug 0))
  (switch Utilities|FlowControl|Switch|SwitchonEnumMV_PanelType (Variables|Settings|GetType)
    (:NewEnumerator0
      _)
    (:NewEnumerator1
      ;[1 1 1] Different Half
      (bind _returnvalue_13 (DynamicMeshActor|AllocateComputeMesh))
      (bind _returnvalue_14 (Class|GeometryScriptLibraryMeshPrimitiveFunctions|AppendBox :TargetMesh _returnvalue_13 :Transform (Math|Transform|MakeTransform (Math|Vector|MakeVector 0.0 _offsetcentery 0.0) "0, 0, 0" "1.000000,1.000000,1.000000") :DimensionX _x :DimensionY _y :DimensionZ _z :Debug 0))
      (bind _returnvalue_15 (GeometryScript|Booleans|ApplyMeshBoolean :TargetMesh _returnvalue_12 :ToolMesh _returnvalue_14 :Operation "Subtract" :Debug 0))
      (bind _returnvalue_16 (DynamicMeshActor|AllocateComputeMesh))
      (bind _returnvalue_17 (Class|GeometryScriptLibraryMeshPrimitiveFunctions|AppendRectangleCompatibility50 :TargetMesh _returnvalue_16 :Transform (Math|Transform|MakeTransform (Math|Vector|MakeVector _offsetcenterx _offsetcentery_2 0.0) "0, 0, 0" "1.000000,1.000000,1.000000") :DimensionX _x_2 :DimensionY _y_2 :Debug 0))
      (bind _returnvalue_18 (Class|GeometryScriptLibraryMeshModelingFunctions|ApplyMeshExtrudeCompatibility5p0 _returnvalue_17 (Utilities|Struct|MakeGeometryScriptMeshExtrudeOptions _extrude "0.000000,0.000000,1.000000" 1.0 true) 0))
      (bind _returnvalue_19 (GeometryScript|Booleans|ApplyMeshBoolean :TargetMesh _returnvalue_15 :ToolMesh _returnvalue_18 :Operation "Union" :Debug 0))
      (bind _returnvalue_20 (DynamicMeshActor|AllocateComputeMesh))
      (bind _returnvalue_21 (Class|GeometryScriptLibraryMeshPrimitiveFunctions|AppendRectangleCompatibility50 :TargetMesh _returnvalue_20 :Transform (Math|Transform|MakeTransform (Math|Vector|MakeVector _offsetx _offsety _offsetz) "0, 0, 0" "1.000000,1.000000,1.000000") :DimensionX _x_3 :DimensionY _y_3 :Debug 0))
      (bind _returnvalue_22 (Class|GeometryScriptLibraryMeshModelingFunctions|ApplyMeshExtrudeCompatibility5p0 _returnvalue_21 (Utilities|Struct|MakeGeometryScriptMeshExtrudeOptions (Variables|Settings|Painting|GetPaintingExtrude) "0.000000,0.000000,1.000000" 1.0 true) 0))
      (bind _returnvalue_23 (GeometryScript|Materials|EnableMaterialIDs _returnvalue_22 0))
      (bind _returnvalue_24 (GeometryScript|Materials|RemapMaterialIDs _returnvalue_23 0 1 0))
      (GeometryScript|Booleans|ApplyMeshBoolean :TargetMesh _returnvalue_19 :ToolMesh _returnvalue_24 :Operation (Variables|Settings|GetOperation) :Debug 0)))
  (bind _returnvalue_25 (Class|GeometryScriptLibraryMeshNormalsFunctions|ComputeSplitNormals _returnvalue_12 (Utilities|Struct|MakeGeometryScriptSplitNormalsOptions true 25.0 false "(bDefaultLayer=True,ExtendedLayerIndex=0)") (Utilities|Struct|MakeGeometryScriptCalculateNormalsOptions true true) 0))
  (Variables|Default|SetDynamicMEsh _returnvalue_25)
  (if (Variables|Settings|Cutter|GetbCustomCutter)
    ;[1 1 1] Cutter
    (Class|GeometryScriptLibraryMeshBooleanFunctions|ApplyMeshPlaneCut (Variables|Default|GetDynamicMEsh) (Math|Transform|MakeTransform (Variables|Settings|Cutter|GetCustomCutter) (Variables|Settings|Cutter|GetCustomCutterRotation) "1.000000,1.000000,1.000000") (Utilities|Struct|MakeGeometryScriptMeshPlaneCutOptions true true false 1.0) 0))
  (if (Variables|Settings|GetbBevelCombine)
    (CallFunction|FnBevel (Variables|Default|GetDynamicMEsh) (Variables|Settings|GetBevelDistanceCombine)))
  (if (Variables|Settings|Mirror|GetbMirror)
    ;[1 1 1] Mirror
    (bind _returnvalue_26 (Class|GeometryScriptLibraryMeshBooleanFunctions|ApplyMeshMirror (Variables|Default|GetDynamicMEsh) (Math|Transform|MakeTransform _location _axis "1.000000,1.000000,1.000000") (Utilities|Struct|MakeGeometryScriptMeshMirrorOptions true true true) 0))
    (Variables|Default|SetDynamicMEsh _returnvalue_26))
  (CallFunction|CleanDegenerateTris (Variables|Default|GetDynamicMEsh) (Variables|Settings|GetSafe%20Normal%20Tolerance) false true)
  (Class|DynamicMeshComponent|ConfigureMaterialSet (Variables|Default|GetDynamicMeshComponent) (Utilities|Array|MakeArray (Variables|Settings|Frame|GetMaterialFrame) (Variables|Settings|Painting|GetMaterialPainting)))
  (DynamicMeshActor|ReleaseAllComputeMeshes))

(fn ConstructionScript
  (|CallParentFunction))

(fn FnBevel
  (params (TargetMesh :type Dynamic%20Mesh%20Object%20Reference) (Options%20Bevel%20Distance :type Float%20%28double-precision%29))
  (return 0))

(fn ApplyMaterials
  (params (Materials :type Array%20of%20Material%20Interface%20Object%20References))
  (Variables|Settings|Frame|SetMaterialFrame (Utilities|Array|Get(acopy) Materials))
  (Variables|Settings|Painting|SetMaterialPainting (Utilities|Array|Get(acopy) Materials 1))
  (return))