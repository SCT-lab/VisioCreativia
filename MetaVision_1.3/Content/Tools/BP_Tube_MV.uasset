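; Geometry Script generator actor that builds a parametric tube or curved wall by revolving a rectangular profile, with optional bevel and complex-as-simple collision.
; RepeaterWall splits the revolve into gapped segments by copying one segment around Z.
; An optional window cutter extrudes rounded rectangles, repeats them radially and subtracts them, or unions them with another material ID for debugging.
; The rebuild finishes with split normals, degenerate-triangle cleanup, material assignment and box-projected UVs.
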(event EventBeginPlay
  (|CallParentFunction) ; This node is disabled and will not be called.\nDrag off pins to build functionality.
)

(event EventTick
  (params (DeltaSeconds :type Float%20%28single-precision%29))
  (|CallParentFunction DeltaSeconds) ; This node is disabled and will not be called.\nDrag off pins to build functionality.
)

(event Events|EventOnRebuildGeneratedMesh
  (params (TargetMesh :type Dynamic%20Mesh%20Object%20Reference))
  (bind _uvscale (Variables|Settings|UVSettings|GetUVScale))
  (Variables|Default|SetDynamicMesh TargetMesh)
  (Utilities|FlowControl|Sequence
    (:then_0
      ;[1 1 1] Create Tube
      (bind _returnvalue (Class|GeometryScriptLibraryMeshPrimitiveFunctions|AppendRevolvePolygon :TargetMesh (Variables|Default|GetDynamicMesh) :PolygonVertices (|MakePolygonVertices_2) :RevolveOptions (|GetRevolveOptions_2) :Radius (|GetRadius_2) :Steps (Variables|Settings|RevolveOptions|GetSteps) :Debug 0))
      (Variables|Default|SetDynamicMesh _returnvalue)
      (if (Variables|Settings|Bevels|GetbBevel)
        ;[1 1 1] Bevel
        (bind _returnvalue_2 (Class|GeometryScriptLibraryMeshModelingFunctions|ApplyMeshPolygroupBevel (Variables|Default|GetDynamicMesh) (Utilities|Struct|MakeGeometryScriptMeshBevelOptions (Variables|Settings|Bevels|GetBevelDistance) false 0 false "(Min=(X=0.000000,Y=0.000000,Z=0.000000),Max=(X=0.000000,Y=0.000000,Z=0.000000),IsValid=False)" "0.000000,0.000000,0.000000|0.000000,0.000000,-0.000000|1.000000,1.000000,1.000000" true) 0))
        (Variables|Default|SetDynamicMesh _returnvalue_2))
      (Utilities|McRepeater)
      (DynamicMeshActor|ReleaseAllComputeMeshes)
      (if (Variables|Settings|Window|GetbWindow)
        (Utilities|McWindowCutter))
      ;[1 1 1] This helps smoothing the Normals
      (bind _returnvalue_3 (Class|GeometryScriptLibraryMeshNormalsFunctions|ComputeSplitNormals :TargetMesh (Variables|Default|GetDynamicMesh) :SplitOptions (Utilities|Struct|MakeGeometryScriptSplitNormalsOptions true 45.0 false "(bDefaultLayer=True,ExtendedLayerIndex=0)") :Debug 0))
      ;[1 1 1] Apply Materials
      (CallFunction|CleanDegenerateTris _returnvalue_3 0.0005 false true)
      (Class|DynamicMeshComponent|ConfigureMaterialSet (Variables|Default|GetDynamicMeshComponent) (Utilities|Array|MakeArray (Variables|Settings|RevolveOptions|GetMaterial) 0))
      (DynamicMeshActor|ReleaseAllComputeMeshes)
      (if (Variables|Default|GetEnableCollison)
        (Class|DynamicMeshComponent|EnableComplexasSimpleCollision (Variables|Default|GetDynamicMeshComponent))))
    (:then_1
      (Class|GeometryScriptLibraryMeshUVFunctions|SetMeshUVsfromBoxProjection :TargetMesh (Variables|Default|GetDynamicMesh) :BoxTransform (Math|Transform|MakeTransform "0, 0, 0" "0, 0, 0" (Math|Vector|MakeVector _uvscale _uvscale _uvscale)) :Debug 0))))

(event EventClearMaterials
  ;[1 1 1] CLEAR MATERIALS
  (Variables|Settings|RevolveOptions|SetMaterial 0)
  ;[1 1 1] Create Tube
  (bind _returnvalue (Class|GeometryScriptLibraryMeshPrimitiveFunctions|AppendRevolvePolygon :TargetMesh (Variables|Default|GetDynamicMesh) :PolygonVertices (|MakePolygonVertices_2) :RevolveOptions (|GetRevolveOptions_2) :Radius (|GetRadius_2) :Steps (Variables|Settings|RevolveOptions|GetSteps) :Debug 0))
  (Variables|Default|SetDynamicMesh _returnvalue)
  (if (Variables|Settings|Bevels|GetbBevel)
    ;[1 1 1] Bevel
    (bind _returnvalue_2 (Class|GeometryScriptLibraryMeshModelingFunctions|ApplyMeshPolygroupBevel (Variables|Default|GetDynamicMesh) (Utilities|Struct|MakeGeometryScriptMeshBevelOptions (Variables|Settings|Bevels|GetBevelDistance) false 0 false "(Min=(X=0.000000,Y=0.000000,Z=0.000000),Max=(X=0.000000,Y=0.000000,Z=0.000000),IsValid=False)" "0.000000,0.000000,0.000000|0.000000,0.000000,-0.000000|1.000000,1.000000,1.000000" true) 0))
    (Variables|Default|SetDynamicMesh _returnvalue_2))
  (Utilities|McRepeater)
  (DynamicMeshActor|ReleaseAllComputeMeshes)
  (if (Variables|Settings|Window|GetbWindow)
    (Utilities|McWindowCutter))
  ;[1 1 1] This helps smoothing the Normals
  (bind _returnvalue_3 (Class|GeometryScriptLibraryMeshNormalsFunctions|ComputeSplitNormals :TargetMesh (Variables|Default|GetDynamicMesh) :SplitOptions (Utilities|Struct|MakeGeometryScriptSplitNormalsOptions true 45.0 false "(bDefaultLayer=True,ExtendedLayerIndex=0)") :Debug 0))
  ;[1 1 1] Apply Materials
  (CallFunction|CleanDegenerateTris _returnvalue_3 0.0005 false true)
  (Class|DynamicMeshComponent|ConfigureMaterialSet (Variables|Default|GetDynamicMeshComponent) (Utilities|Array|MakeArray (Variables|Settings|RevolveOptions|GetMaterial) 0))
  (DynamicMeshActor|ReleaseAllComputeMeshes)
  (if (Variables|Default|GetEnableCollison)
    (Class|DynamicMeshComponent|EnableComplexasSimpleCollision (Variables|Default|GetDynamicMeshComponent))))

(fn ConstructionScript
  (|CallParentFunction))

(fn FnRepeater
  (params (InputPin :type Dynamic%20Mesh%20Object%20Reference) (Instances :type Integer))
  (bind _returnvalue (DynamicMeshActor|AllocateComputeMesh))
  (bind _copytomeshout (GeometryScript|Decomposition|CopyMeshtoMesh InputPin _returnvalue 0))
  (bind _returnvalue_2 (Class|GeometryScriptLibraryMeshBasicEditFunctions|AppendMeshRepeated InputPin _copytomeshout (Math|Transform|MakeTransform "0, 0, 0" (Math|Rotator|MakeRotator 0.0 0.0 (|GetRotationRate_2)) "1.000000,1.000000,1.000000") (- Instances 1) true false "(CombineMode=EnableAllMatching)" 0))
  (return _returnvalue_2))