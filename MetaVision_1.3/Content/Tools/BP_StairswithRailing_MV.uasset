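; Geometry Script generated-mesh tool that builds a linear staircase with optional side railings, using fixed or adaptive step counts.
; On rebuild it appends stairs, optionally bevels them, and can set convex-hull collision from an extruded simplified profile.
; Railings are boxes plane-cut at the slope pitch derived from component bounds, with bevelled tops and separate material IDs.
; It finishes by applying materials, enabling complex-as-simple collision and box-projecting UVs.
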(event `self.ClearMaterials`
  (bind _num_steps (`self.Num Steps`))
  (bind (_handle_x _handle_y _handle_z) (`KismetMathLibrary.BreakVector` (`self.Handle`)))
  (bind (_handle_x_2 _handle_y_2 _handle_z_2) (`KismetMathLibrary.BreakVector` (`self.Handle`)))
  (bind (_handle_x_3 _handle_y_3 _handle_z_3) (`KismetMathLibrary.BreakVector` (`self.Handle`)))
  (bind _stepheight (`self.StepHeight`))
  (bind _railingcutterangle (`self.RailingCutterAngle`))
  (bind _railingcutterangle_2 (`self.RailingCutterAngle`))
  (bind _target_mesh (`self.Target Mesh`))
  (bind _railingcutterangle_3 (`self.RailingCutterAngle`))
  (bind _railingcutterangle_4 (`self.RailingCutterAngle`))
  (bind _floating (`self.Floating`))
  (bind (_stairsbounds_x _stairsbounds_y _stairsbounds_z) (`KismetMathLibrary.BreakVector` (`self.StairsBounds`)))
  (bind (_stairsbounds_x_2 _stairsbounds_y_2 _stairsbounds_z_2) (`KismetMathLibrary.BreakVector` (`self.StairsBounds`)))
  (bind (_stairsbounds_x_3 _stairsbounds_y_3 _stairsbounds_z_3) (`KismetMathLibrary.BreakVector` (`self.StairsBounds`)))
  (bind (_stairsbounds_x_4 _stairsbounds_y_4 _stairsbounds_z_4) (`KismetMathLibrary.BreakVector` (`self.StairsBounds`)))
  (bind (_origin _boxextent) (`KismetSystemLibrary.GetComponentBounds` (`self.DynamicMeshComponent`)))
  (bind (_returnvalue_min _returnvalue_max) (break `Box` (`GeometryScriptLibrary_MeshQueryFunctions.GetMeshBoundingBox` (`self.Target Mesh`))))
  (bind _returnvalue (/ _stairsbounds_z_4 2.0))
  (bind _returnvalue_2 (/ _stairsbounds_z_2 2.0))
  (bind _returnvalue_3 (`KismetMathLibrary.FTrunc` (/ _handle_x_3 _stepheight)))
  (bind _returnvalue_4 (+ (/ _stairsbounds_z_3 2.0) (/ (`self.RailingWallHeight`) 2.0) (`self.RailingTopperDimension`)))
  (bind _returnvalue_5 (+ (/ _stairsbounds_z 2.0) (/ (`self.RailingWallHeight`) 2.0) (`self.RailingTopperDimension`)))
  (bind (_returnvalue_roll _returnvalue_pitch) (`KismetMathLibrary.BreakRotator` (`KismetMathLibrary.FindRelativeLookAtRotation` (`KismetMathLibrary.MakeTransform` (0.0 0.0 0.0)) (`KismetMathLibrary.MakeVector` (.x _boxextent) 0.0 (.z _boxextent)))))
  ;[1 1 1] CLEAR MATERIALS
  (set `self.Material` null)
  (`DynamicMeshComponent.ConfigureMaterialSet` (`self.DynamicMeshComponent`) (`|MakeArray` (`self.Material`)))
  (switch `/MetaVision/Tools/Enums/EnumMV_StairConstructionType` (`self.Type`) :!label _label
    (:`NewEnumerator0`
      ;[1 1 1] Generate the Stairs
      (bind _returnvalue_6 (`GeometryScriptLibrary_MeshPrimitiveFunctions.AppendLinearStairs` (stale `self.OnRebuildGeneratedMesh` TargetMesh) (struct) (`KismetMathLibrary.MakeTransform` (`KismetMathLibrary.MakeVector` 0.0 (/ _handle_y_3 2.0))) _handle_y_3 (/ _handle_z_3 _returnvalue_3) _stepheight _returnvalue_3 _floating null))
      (set `self.Target Mesh` _returnvalue_6))
    (:`NewEnumerator1`
      (bind _returnvalue_7 (`GeometryScriptLibrary_MeshPrimitiveFunctions.AppendLinearStairs` (stale `self.OnRebuildGeneratedMesh` TargetMesh) (struct) (`KismetMathLibrary.MakeTransform` (`KismetMathLibrary.MakeVector` 0.0 (/ _handle_y 2.0))) _handle_y (/ _handle_z _num_steps) (/ _handle_x _num_steps) _num_steps _floating null))
      (set `self.Target Mesh` _returnvalue_7)))
  (if (`self.bBevel`)
    ;[1 1 1] Bevel
    (`GeometryScriptLibrary_MeshPolygroupFunctions.ComputePolygroupsFromAngleThreshold` _target_mesh (make `GeometryScriptGroupLayer` true) 25.0 2 null)
    (bind _returnvalue_8 (`GeometryScriptLibrary_MeshModelingFunctions.ApplyMeshPolygroupBevel` _target_mesh (make `GeometryScriptMeshBevelOptions` (`self.DistanceBevel`) true) null))
    (bind _returnvalue_9 (`GeometryScriptLibrary_MeshNormalsFunctions.ComputeSplitNormals` _returnvalue_8 (make `GeometryScriptSplitNormalsOptions` true 25.0) (make `GeometryScriptCalculateNormalsOptions` true) null))
    (set `self.Target Mesh` _returnvalue_9))
  (if (`self.bSimplifiedCollision`)
    ;[1 1 1] Simplified Collision Generation
    (bind _returnvalue_10 (`self.AllocateComputeMesh`))
    (set `self.Simplified` _returnvalue_10)
    (bind _returnvalue_11 (`GeometryScriptLibrary_MeshPrimitiveFunctions.AppendSimpleExtrudePolygon` (`self.Simplified`) (struct) (`KismetMathLibrary.MakeTransform` (0.0 0.0 0.0)) (select `bool` (`self.bTriangle`) :`true` (select `byte` (`self.Type`) :`0` _ :`1` _ :!type "Array of Vector2D Structure")) _handle_y_2 0 true "Base" null))
    (set `self.Simplified` _returnvalue_11)
    (if (`self.bPreviewSimplified(turnOFFBEFOREBAKE)`)
      ;;[1 1 1] This is just to preview temporary the Collision Mesh
      (bind _returnvalue_12 (`GeometryScriptLibrary_MeshMaterialFunctions.RemapMaterialIDs` (`self.Simplified`) 0 1 null))
      (bind _returnvalue_13 (`GeometryScriptLibrary_MeshBasicEditFunctions.AppendMesh` (`self.Target Mesh`) _returnvalue_12 (struct) false (struct :`CombineMode` "EnableAllMatching") null))
      (set `self.Target Mesh` _returnvalue_13)
      (else
        (bind _returnvalue_14 (`GeometryScriptLibrary_CollisionFunctions.SetDynamicMeshCollisionFromMesh` (`self.Simplified`) (`self.DynamicMeshComponent`) (make `GeometryScriptCollisionFromMeshOptions` false "ConvexHulls" false false false 1.0 false 25 1 0.5 0.0 0.1 0.1 "Z" false) null))
        (set `self.Target Mesh` _returnvalue_14)))
    (else
      ;[1 1 1] Don't simplified the Collision
      (`GeometryScriptLibrary_CollisionFunctions.ResetDynamicMeshCollision` (`self.DynamicMeshComponent`) false null)))
  (`self.CleanDegenerateTris` (`self.Target Mesh`))
  (`self.ReleaseAllComputeMeshes`)
  ;[1 1 1] GET THE ANGLE FOR THE RAILING
  (set `self.RailingCutterAngle` _returnvalue_pitch)
  ;[1 1 1] GET THE BOUNDS OF THE STAIRCASE
  (set `self.StairsBounds` _returnvalue_max)
  (if (`self.makeLeftRailing?`)
    ;[1 1 1] MAKE THE LEFT SIDE RAILING WALL / GLASS
    (bind _returnvalue_15 (`self.AllocateComputeMesh`))
    (bind _returnvalue_16 (`GeometryScriptLibrary_MeshPrimitiveFunctions.AppendBox` _returnvalue_15 (struct) (`KismetMathLibrary.MakeTransform` (0.0 0.0 0.0)) _stairsbounds_x_2 (`self.RailingWallWidth`) (* _stairsbounds_z_2 2.0) 0 0 0 "Base" null))
    (bind _returnvalue_17 (`GeometryScriptLibrary_MeshBooleanFunctions.ApplyMeshPlaneCut` _returnvalue_16 (`KismetMathLibrary.MakeTransform` (`KismetMathLibrary.MakeVector` 0.0 0.0 (+ _returnvalue_2 (`self.RailingWallHeight`))) (`KismetMathLibrary.MakeRotator` 0.0 _railingcutterangle_3)) (make `GeometryScriptMeshPlaneCutOptions` true) null))
    (bind _returnvalue_18 (`GeometryScriptLibrary_MeshBooleanFunctions.ApplyMeshPlaneCut` _returnvalue_17 (`KismetMathLibrary.MakeTransform` (`KismetMathLibrary.MakeVector` 0.0 0.0 _returnvalue_2) (`KismetMathLibrary.MakeRotator` 0.0 (+ _railingcutterangle_3 180.0))) (make `GeometryScriptMeshPlaneCutOptions` true) null))
    (bind _returnvalue_19 (`GeometryScriptLibrary_MeshMaterialFunctions.RemapMaterialIDs` _returnvalue_18 0 1 null))
    (bind _returnvalue_20 (`GeometryScriptLibrary_MeshBasicEditFunctions.AppendMesh` (`self.Target Mesh`) _returnvalue_19 (`KismetMathLibrary.MakeTransform` (`KismetMathLibrary.MakeVector` (/ _stairsbounds_x_2 2.0) (+ (/ (`self.RailingWallWidth`) 2.0) 1.0))) false (struct :`CombineMode` "EnableAllMatching") null))
    (set `self.Target Mesh` _returnvalue_20)
    ;[1 1 1] MAKE LEFT SIDE RAILING TOP
    (bind _returnvalue_21 (`self.AllocateComputeMesh`))
    (bind _returnvalue_22 (`GeometryScriptLibrary_MeshPrimitiveFunctions.AppendBox` _returnvalue_21 (struct) (`KismetMathLibrary.MakeTransform` (0.0 0.0 0.0)) (* _stairsbounds_x_3 1.05) (`self.RailingTopperDimension`) (* _stairsbounds_z_3 2.0) 0 0 0 "Base" null))
    (bind _returnvalue_23 (`GeometryScriptLibrary_MeshBooleanFunctions.ApplyMeshPlaneCut` _returnvalue_22 (`KismetMathLibrary.MakeTransform` (`KismetMathLibrary.MakeVector` 0.0 0.0 _returnvalue_4) (`KismetMathLibrary.MakeRotator` 0.0 _railingcutterangle_4)) (make `GeometryScriptMeshPlaneCutOptions` true) null))
    (bind _returnvalue_24 (`GeometryScriptLibrary_MeshBooleanFunctions.ApplyMeshPlaneCut` _returnvalue_23 (`KismetMathLibrary.MakeTransform` (`KismetMathLibrary.MakeVector` 0.0 0.0 (- _returnvalue_4 (`self.RailingTopperDimension`))) (`KismetMathLibrary.MakeRotator` 0.0 (+ _railingcutterangle_4 180.0))) (make `GeometryScriptMeshPlaneCutOptions` true) null))
    (bind _returnvalue_25 (`GeometryScriptLibrary_MeshModelingFunctions.ApplyMeshPolygroupBevel` _returnvalue_24 (make `GeometryScriptMeshBevelOptions` (`self.RailingTopBevelAmount`)) null))
    (bind _returnvalue_26 (`GeometryScriptLibrary_MeshNormalsFunctions.ComputeSplitNormals` _returnvalue_25 (struct) (struct) null))
    (bind _returnvalue_27 (`GeometryScriptLibrary_MeshMaterialFunctions.RemapMaterialIDs` _returnvalue_26 0 2 null))
    (bind _returnvalue_28 (`GeometryScriptLibrary_MeshBasicEditFunctions.AppendMesh` (`self.Target Mesh`) _returnvalue_27 (`KismetMathLibrary.MakeTransform` (`KismetMathLibrary.MakeVector` (/ _stairsbounds_x_3 2.0) (+ (/ (`self.RailingWallWidth`) 2.0) 1.0) (* (`self.RailingWallHeight`) 0.5))) false (struct :`CombineMode` "EnableAllMatching") null))
    (set `self.Target Mesh` _returnvalue_28))
  (if (`self.makeRightRailing?`)
    ;[1 1 1] MAKE THE RIGHT SIDE RAILING WALL / GLASS
    (bind _returnvalue_29 (`self.AllocateComputeMesh`))
    (bind _returnvalue_30 (`GeometryScriptLibrary_MeshPrimitiveFunctions.AppendBox` _returnvalue_29 (struct) (`KismetMathLibrary.MakeTransform` (0.0 0.0 0.0)) _stairsbounds_x_4 (`self.RailingWallWidth`) (* _stairsbounds_z_4 2.0) 0 0 0 "Base" null))
    (bind _returnvalue_31 (`GeometryScriptLibrary_MeshBooleanFunctions.ApplyMeshPlaneCut` _returnvalue_30 (`KismetMathLibrary.MakeTransform` (`KismetMathLibrary.MakeVector` 0.0 0.0 (+ _returnvalue (`self.RailingWallHeight`))) (`KismetMathLibrary.MakeRotator` 0.0 _railingcutterangle)) (make `GeometryScriptMeshPlaneCutOptions` true) null))
    (bind _returnvalue_32 (`GeometryScriptLibrary_MeshBooleanFunctions.ApplyMeshPlaneCut` _returnvalue_31 (`KismetMathLibrary.MakeTransform` (`KismetMathLibrary.MakeVector` 0.0 0.0 _returnvalue) (`KismetMathLibrary.MakeRotator` 0.0 (+ _railingcutterangle 180.0))) (make `GeometryScriptMeshPlaneCutOptions` true) null))
    (bind _returnvalue_33 (`GeometryScriptLibrary_MeshMaterialFunctions.RemapMaterialIDs` _returnvalue_32 0 1 null))
    (bind _returnvalue_34 (`GeometryScriptLibrary_MeshBasicEditFunctions.AppendMesh` (`self.Target Mesh`) _returnvalue_33 (`KismetMathLibrary.MakeTransform` (`KismetMathLibrary.MakeVector` (/ _stairsbounds_x_4 2.0) (- _stairsbounds_y_4 (+ (/ (`self.RailingWallWidth`) 2.0) 1.0)))) false (struct :`CombineMode` "EnableAllMatching") null))
    (set `self.Target Mesh` _returnvalue_34)
    ;[1 1 1] MAKE RIGHT SIDE RAILING TOP
    (bind _returnvalue_35 (`self.AllocateComputeMesh`))
    (bind _returnvalue_36 (`GeometryScriptLibrary_MeshPrimitiveFunctions.AppendBox` _returnvalue_35 (struct) (`KismetMathLibrary.MakeTransform` (0.0 0.0 0.0)) (* _stairsbounds_x 1.05) (`self.RailingTopperDimension`) (* _stairsbounds_z 2.0) 0 0 0 "Base" null))
    (bind _returnvalue_37 (`GeometryScriptLibrary_MeshBooleanFunctions.ApplyMeshPlaneCut` _returnvalue_36 (`KismetMathLibrary.MakeTransform` (`KismetMathLibrary.MakeVector` 0.0 0.0 _returnvalue_5) (`KismetMathLibrary.MakeRotator` 0.0 _railingcutterangle_2)) (make `GeometryScriptMeshPlaneCutOptions` true) null))
    (bind _returnvalue_38 (`GeometryScriptLibrary_MeshBooleanFunctions.ApplyMeshPlaneCut` _returnvalue_37 (`KismetMathLibrary.MakeTransform` (`KismetMathLibrary.MakeVector` 0.0 0.0 (- _returnvalue_5 (`self.RailingTopperDimension`))) (`KismetMathLibrary.MakeRotator` 0.0 (+ _railingcutterangle_2 180.0))) (make `GeometryScriptMeshPlaneCutOptions` true) null))
    (bind _returnvalue_39 (`GeometryScriptLibrary_MeshModelingFunctions.ApplyMeshPolygroupBevel` _returnvalue_38 (make `GeometryScriptMeshBevelOptions` (`self.RailingTopBevelAmount`)) null))
    (bind _returnvalue_40 (`GeometryScriptLibrary_MeshNormalsFunctions.ComputeSplitNormals` _returnvalue_39 (struct) (struct) null))
    (bind _returnvalue_41 (`GeometryScriptLibrary_MeshMaterialFunctions.RemapMaterialIDs` _returnvalue_40 0 2 null))
    (bind _returnvalue_42 (`GeometryScriptLibrary_MeshBasicEditFunctions.AppendMesh` (`self.Target Mesh`) _returnvalue_41 (`KismetMathLibrary.MakeTransform` (`KismetMathLibrary.MakeVector` (/ _stairsbounds_x 2.0) (- _stairsbounds_y (+ (/ (`self.RailingWallWidth`) 2.0) 1.0)) (* (`self.RailingWallHeight`) 0.5))) false (struct :`CombineMode` "EnableAllMatching") null))
    (set `self.Target Mesh` _returnvalue_42))
  ;[1 1 1] Apply Material
  (`DynamicMeshComponent.ConfigureMaterialSet` (`self.DynamicMeshComponent`) (`|MakeArray` (`self.StairsMaterial`) (`self.RailingMaterial`) (`self.RailingTopMaterial`)))
  (`self.ReleaseAllComputeMeshes`)
  (`DynamicMeshComponent.EnableComplexAsSimpleCollision` (`self.DynamicMeshComponent`)))

(event `self.OnRebuildGeneratedMesh`
  (params (TargetMesh :type "DynamicMesh Object Reference"))
  (bind _uv_scale (`self.UV Scale`))
  (`|ExecutionSequence`
    (:`then_0`
      (goto _label))
    (:`then_1`
      (`GeometryScriptLibrary_MeshUVFunctions.SetMeshUVsFromBoxProjection` (`self.Target Mesh`) 0 (`KismetMathLibrary.MakeTransform` (0.0 0.0 0.0) (struct) (`KismetMathLibrary.MakeVector` _uv_scale _uv_scale _uv_scale)) (struct) 2 null))))

(fn `ApplyMaterials`
  (params (Materials :type "Array of MaterialInterface Object Reference (by ref)"))
  (set `self.Material` (`|GetArrayItem` Materials))
  (return))

(fn `UserConstructionScript`
  (`parent.UserConstructionScript`))