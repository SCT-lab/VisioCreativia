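; BP_Painting1 is an interactable painting that toggles its Painting component's visibility with the E key.
; Overlap with its Sphere by BP_FirstPersonCharacter shows or hides the interaction prompt and sets an in-range flag.
; It reads E directly through player 0 input, leaving Interact empty.
; A FlipFlop alternates showing, which requires range and hides the prompt, with unconditional hiding, so out-of-range presses still advance the toggle.
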(event `self.ReceiveBeginPlay`
  (`self.EnableInput` (`GameplayStatics.GetPlayerController` 0)))

(event `self.Sphere.OnComponentBeginOverlap`
  (params (OverlappedComponent :type "PrimitiveComponent Object Reference") (OtherActor :type "Actor Object Reference") (OtherComp :type "PrimitiveComponent Object Reference") (OtherBodyIndex :type Integer) (bFromSweep :type Boolean) (SweepResult :type "HitResult Structure (by ref)"))
  (cast `/Game/FirstPerson/Blueprints/BP_FirstPersonCharacter` OtherActor)
  (`SceneComponent.SetVisibility` (`self.InteractionPromt`) true false)
  (set `self.WidgetVisibile` true))

(event `self.Interact`)

(event `self.Sphere.OnComponentEndOverlap`
  (params (OverlappedComponent :type "PrimitiveComponent Object Reference") (OtherActor :type "Actor Object Reference") (OtherComp :type "PrimitiveComponent Object Reference") (OtherBodyIndex :type Integer))
  (cast `/Game/FirstPerson/Blueprints/BP_FirstPersonCharacter` OtherActor)
  (`SceneComponent.SetVisibility` (`self.InteractionPromt`) false false)
  (set `self.WidgetVisibile` false))

(event `Key|E`
  (params (Key :type "Key Structure"))
  (bind _painting (`self.Painting`))
  (:`Pressed`
    (`/Engine/EditorBlueprintResources/StandardMacros.FlipFlop`
      (:`A`
        (if (`self.WidgetVisibile`)
          (`SceneComponent.SetVisibility` _painting true false)
          (bind _output_get (set `self.Widget1Visible` true))
          (if _output_get
            (`SceneComponent.SetVisibility` (`self.InteractionPromt`) false false))))
      (:`B`
        (if true
          (`SceneComponent.SetVisibility` _painting false false)
          (set `self.Widget1Visible` false))))))

(fn `UserConstructionScript`)